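; AK-47 weapon item Blueprint that supplies the gun's name and a focusable in-world info widget.
; On BeginPlay it sets the name and formats a Spanish description from its base damage and rate of fire.
; Each Tick it turns the widget component toward the player's eye viewpoint with a slight pitch offset, like a billboard.
; StartFocusItem and EndFocusItem only toggle the focus flag and report success.
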(event `self.ReceiveBeginPlay`
  (set `self.Name` "AK-47")
  (set `self.Descripcion` (`|FormatText` "Arma de medio alcance. \nDaño: {Danio} \nRatio de disparo: {Ratio} \nRetroceso: Medio-Alto" (`self.BaseDamage`) (`self.RateOfFire`))))

(event `self.ReceiveTick`
  (params (DeltaSeconds :type "Float (single-precision)"))
  (bind _actorwidgetcomp (`self.ActorWidgetComp`))
  (bind (_returnvalue_roll _returnvalue_pitch _returnvalue_yaw) (`KismetMathLibrary.BreakRotator` (`KismetMathLibrary.FindLookAtRotation` (`SceneComponent.K2_GetComponentLocation` _actorwidgetcomp) (`self.GetActorEyesViewPoint` (`GameplayStatics.GetPlayerCharacter` 0)))))
  (`SceneComponent.K2_SetWorldRotation` _actorwidgetcomp (`KismetMathLibrary.MakeRotator` _returnvalue_roll (+ _returnvalue_pitch 10.0) _returnvalue_yaw) false false))

(fn `EndFocusItem`
  (returns (ReturnValue :type Boolean))
  (set `self.bIsFocused` false)
  (return true))

(fn `StartFocusItem`
  (returns (ReturnValue :type Boolean))
  (set `self.bIsFocused` true)
  (return true))

(fn `UserConstructionScript`)