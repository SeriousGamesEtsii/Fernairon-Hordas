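; AI companion that, on BeginPlay, runs the BT_AICompanion behavior tree and picks a player to accompany.
; It steps through player pawns by index until it finds an SCharacter whose GetCurrentCompanion returns zero, then stores that pawn in the CompanionPlayer blackboard key.
; The search stops without assigning a player if a pawn fails the SCharacter cast.
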(event `self.ReceiveBeginPlay`
  (`AIController.RunBehaviorTree` (`AIBlueprintHelperLibrary.GetAIController` self) "/Game/AICompanion/BT_AICompanion.BT_AICompanion")
  (bind _asscharacter (cast `SCharacter` (`GameplayStatics.GetPlayerPawn` (`self.IndexPlayer`)) :!label _label))
  (bind _returnvalue (`self.GetCurrentCompanion` _asscharacter))
  (if (== _returnvalue 0)
    (`BlackboardComponent.SetValueAsObject` (`AIBlueprintHelperLibrary.GetBlackboard` self) "CompanionPlayer" (`GameplayStatics.GetPlayerPawn` (`self.IndexPlayer`)))
    (else
      (set `self.IndexPlayer` (+ (`self.IndexPlayer`) 1))
      (goto _label))))

(fn `UserConstructionScript`)