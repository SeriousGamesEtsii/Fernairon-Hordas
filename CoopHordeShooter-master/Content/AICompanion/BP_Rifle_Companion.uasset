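; BP_Rifle_Companion is the AI companion's rifle, whose base damage grows as the game's rounds progress.
; Every Tick it compares the SGameModeBase round number with its InterruptorF counter.
; On a match it prints the current damage, adds twice the round number to it and increments the counter, so each matched round applies the bonus once.
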(event `self.ReceiveTick`
  (params (DeltaSeconds :type "Float (single-precision)"))
  (bind _returnvalue (`self.GetBaseDamage` self))
  (bind _assgame_mode_base (cast `SGameModeBase` (`GameplayStatics.GetGameMode`)))
  (bind _returnvalue_2 (`SGameModeBase.GetNumRound` _assgame_mode_base))
  (if (== _returnvalue_2 (`self.interruptorF`))
    (set `self.interruptor` true)
    (`KismetSystemLibrary.PrintString` (`KismetStringLibrary.Conv_DoubleToString` _returnvalue))
    (if (`self.interruptor`)
      (bind _assgame_mode_base_2 (cast `SGameModeBase` (`GameplayStatics.GetGameMode`)))
      (bind _returnvalue_3 (`SGameModeBase.GetNumRound` _assgame_mode_base_2))
      (`self.SetBaseDamage` self (+ (`KismetMathLibrary.Conv_IntToDouble` (* _returnvalue_3 2)) _returnvalue))
      (set `self.interruptor` false)
      (set `self.interruptorF` (+ (`self.interruptorF`) 1)))))

(fn `UserConstructionScript`)